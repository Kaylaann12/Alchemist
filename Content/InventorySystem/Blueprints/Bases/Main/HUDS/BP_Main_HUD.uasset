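; BP_Main_HUD is the main HUD for the inventory system, owning the player's HUD and inventories widgets.
; On BeginPlay it sets game-only input, then creates both widgets and adds them to the viewport.
; Events forward interaction messages and inventory updates to those widgets.
; Toggling the inventory flips widget visibility, switching input mode and mouse cursor, and refreshes the player's inventory when shown.
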(event EventBeginPlay
  (Utilities|FlowControl|Sequence
    (:then_0
      ;[1 1 1] Focusing on the game
      (Input|SetInputModeGameOnly (Game|Player|GetOwningPlayerController) false))
    (:then_1
      ;[1 1 1] Creating and adding the HUD widget to the viewport
      (bind _returnvalue (UserInterface|CreateWidget "/Game/InventorySystem/Widgets/HUD/WB_HUD.WB_HUD_C" (Game|Player|GetOwningPlayerController)))
      (bind _output_get (Variables|Default|SetHUD_WB _returnvalue))
      (UserInterface|Viewport|AddtoViewport _output_get 0))
    (:then_2
      ;[1 1 1] Creating the inventories widget
      (bind _returnvalue_2 (UserInterface|CreateWidget "/Game/InventorySystem/Widgets/Inventory/WB_Inventories.WB_Inventories_C" (Game|Player|GetOwningPlayerController)))
      (bind _output_get_2 (Variables|Default|SetInventories_HUD _returnvalue_2))
      (UserInterface|Viewport|AddtoViewport _output_get_2 0))))

(event EventSetMainPlayerInventory
  (params (Inventory :type BPC%20Inventory%20Object%20Reference))
  ;[1 1 1] Setting main player inventory
  (bind _inventories_hud (Variables|Default|GetInventories_HUD)
    (:then
      (Default|SetMainPlayerInventory _inventories_hud Inventory))
    (:else)))

(event EventUpdateMainPlayerSlots
  ;[1 1 1] Update player's main slots
  (Default|UpdatePlayerMainInventory (Variables|Default|GetInventories_HUD)))

(event EventShowInteractionMessage
  (params (Interaction_Message :type Text))
  ;[1 1 1] Show interaction message
  (Default|ShowInteractionMessage (Variables|Default|GetHUD_WB) Interaction_Message))

(event EventHideInteractionMessage
  ;[1 1 1] Hide interaction message
  (Default|HideInteractionMessage (Variables|Default|GetHUD_WB)))

(event EventTogglePlayerInventory
  (bind _inventories_hud (Variables|Default|GetInventories_HUD))
  ;[1 1 1] Toggle player's inventory
  (bind _visible_ (CallFunction|ToggleWidgetVisibility _inventories_hud))
  (if _visible_
    (Default|UpdatePlayerMainInventory _inventories_hud)))

(fn ConstructionScript)

(fn ToggleWidgetVisibility
  (params (Widget :type User%20Widget%20Object%20Reference))
  (bind _returnvalue (Game|Player|GetOwningPlayerController))
  (bind _returnvalue_2 (Game|Player|GetOwningPlayerController))
  (if (Widget|IsVisible Widget)
    (Widget|SetVisibility Widget "Collapsed")
    (Input|SetInputModeGameOnly _returnvalue_2 false)
    (Variables|/Script/Engine.PlayerController|SetbShowMouseCursor _returnvalue_2 false)
    (return false)
    (else
      (Widget|SetVisibility Widget "Visible")
      (Input|SetInputModeGameandUI _returnvalue Widget "DoNotLock" true false)
      (Variables|/Script/Engine.PlayerController|SetbShowMouseCursor _returnvalue true)
      (return true))))