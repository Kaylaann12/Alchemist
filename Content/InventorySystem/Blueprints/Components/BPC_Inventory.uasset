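; Inventory component that holds an array of item slots, filled with empty slots at BeginPlay, and registers itself with the HUD when it is the player inventory.
; AddItem looks up item info in the database and places units one at a time, topping up stacks below max size before taking empty slots.
; It prints a message when no slot is free and returns the amount actually added.
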(event EventBeginPlay
  (CallFunction|InitializeInventory))

(fn InitializeInventory
  (for _index (range 1 (Variables|Default|GetSlots_Count))
    (Utilities|Array|Add (Variables|Default|GetContent) (Utilities|Struct|MakeStruct_Inventory_Slot "None" 0 false)))
  (switch Utilities|FlowControl|Switch|SwitchonEnum_Inventory_Types (Variables|Default|GetInventory_Type)
    (:NewEnumerator0
      (Class|BPIHUD|SetMainPlayerInventory(Message) (HUD|GetHUD (Game|GetPlayerController 0)) self))))

(fn FindEmptySlot
  (for (_array_element _array_index) (Variables|Default|GetContent)
    (if (not (.Occupied? (Utilities|Struct|BreakStruct_Inventory_Slot _array_element)))
      (return true _array_index)))
  (return false -1))

(fn FindAvailableSlotwithItem
  (params (Item_ID_To_Add :type Name))
  (bind (_success_ _item_infos) (CallFunction|GetItemInfofromDB Item_ID_To_Add))
  (if _success_
    (for (_array_element _array_index) (Variables|Default|GetContent)
      (if (== Item_ID_To_Add (.Item_ID (Utilities|Struct|BreakStruct_Inventory_Slot _array_element)))
        (if (<= (+ (.Amount (Utilities|Struct|BreakStruct_Inventory_Slot _array_element)) 1) (.Max_Stack_Size (Utilities|Struct|BreakStruct_Items _item_infos)))
          (return true _array_index))))
    (return false -1)))

(fn AddItemtoEmptySlot
  (params (Slot_Index :type Integer) (Item_ID_To_Add :type Name) (Actor_Class_To_Class :type Actor%20Soft%20Class%20Reference))
  (Utilities|Array|SetArrayElem (Variables|Default|GetContent) Slot_Index (Utilities|Struct|MakeStruct_Inventory_Slot Item_ID_To_Add 1 true Actor_Class_To_Class))
  (return true))

(fn AddItemtoSlotStack
  (params (Slot_Index :type Integer))
  (bind _content (Variables|Default|GetContent))
  (bind _output (Utilities|Array|Get(acopy) _content Slot_Index))
  (bind (_item_id _amount _occupied_ _actor_class) (Utilities|Struct|BreakStruct_Inventory_Slot _output))
  (Utilities|Array|SetArrayElem (Variables|Default|GetContent) Slot_Index (Utilities|Struct|MakeStruct_Inventory_Slot _item_id (+ _amount 1) _occupied_ _actor_class))
  (return true))

(fn AddItem
  (params (Item_ID_To_Add :type Name) (Amount_To_Add :type Integer))
  (bind (_success_ _item_infos) (CallFunction|GetItemInfofromDB Item_ID_To_Add))
  ;[1 1 1] Setting the initial values
  (LocalVariables|SetItem_Left Amount_To_Add)
  (if _success_
    (LocalVariables|SetItem_Infos _item_infos)
    (for _index (range 1 Amount_To_Add)
      ;[1 1 1] If the item is stackableor not
      (if (.stackacble? (LocalVariables|GetItem_Infos))
        ;[1 1 1] Finding a slot with the item
        (bind (_success__2 _slot_index) (Helper|FindAvailableSlotwithItem Item_ID_To_Add))
        (if _success__2
          ;[1 1 1] Adding item to the same slot
          (bind _success__3 (Helper|AddItemtoSlotStack _slot_index))
          (if _success__3
            (LocalVariables|SetItem_Left (- (LocalVariables|GetItem_Left) 1)))
          (else
            ;[1 1 1] Adding item to an empty slot in case we didn't find a slot with the same item or if it is already full
            (bind (_success__4 _slot_index_2) (Helper|FindEmptySlot))
            (if _success__4
              (bind _success__5 (Helper|AddItemtoEmptySlot _slot_index_2 Item_ID_To_Add (.actor_class (LocalVariables|GetItem_Infos))))
              (if _success__5
                (LocalVariables|SetItem_Left (- (LocalVariables|GetItem_Left) 1)))
              (else
                (Development|PrintString "Inventory Full")))))
        (else
          ;[1 1 1] Finding an empty slot
          (bind (_success__6 _slot_index_3) (Helper|FindEmptySlot))
          (if _success__6
            ;[1 1 1] Adding item to an empty slot if the item is not stackable
            (bind _success__7 (Helper|AddItemtoEmptySlot _slot_index_3 Item_ID_To_Add (.actor_class (LocalVariables|GetItem_Infos))))
            (if _success__7
              (LocalVariables|SetItem_Left (- (LocalVariables|GetItem_Left) 1)))
            (else
              (Development|PrintString "Inventory Full"))))))
    ;[1 1 1] Return the amount of item added after finishing adding the necessary item
    (return (- Amount_To_Add (LocalVariables|GetItem_Left)))))